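; BP_AutomaticRifle is a rifle weapon that a BP_MainUnit picks up on interact and that reloads on BeginPlay.
; Shoot runs a debug-drawn Visibility line trace from the ShootPoint toward a distant point along the owning unit's camera forward vector.
; A hit spawns a particle emitter at the impact and checks the hit actor for an ability system component, with no action following that check yet.
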(event EventBeginPlay
  (Class|WeaponBase|Reload))

(event EventInteract
  (params (Interactor :type Actor%20Object%20Reference))
  (bind _asbp_main_unit (Utilities|Casting|CastToBP_MainUnit Interactor))
  (Default|PickUpWeapon _asbp_main_unit self))

(event EventShoot
  (bind _asbp_main_unit (Utilities|Casting|CastToBP_MainUnit (Components|GetOwner)))
  (bind (_outhit _returnvalue) (Collision|LineTraceByChannel (Transformation|GetWorldLocation (Variables|Default|GetShootPoint)) (+ (Transformation|GetWorldLocation (Variables|/Game/TestGame/Blueprints/Characters/BP_MainUnit.BP_MainUnit_C|GetCurrentCamera _asbp_main_unit)) (* (Math|Vector|GetForwardVector (Variables|/Game/TestGame/Blueprints/Characters/BP_MainUnit.BP_MainUnit_C|GetCurrentCamera _asbp_main_unit)) 1e+04)) "TraceTypeQuery1" false 0 "ForDuration"))
  (if _returnvalue
    (Effects|SpawnEmitteratLocation "/Engine/Tutorial/SubEditors/TutorialAssets/TutorialParticleSystem.TutorialParticleSystem" (.Location (Collision|BreakHitResult _outhit)))
    (Utilities|IsValid (Ability|GetAbilitySystemComponent (.HitActor (Collision|BreakHitResult _outhit))))))

(fn ConstructionScript)