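; BP_Player is a player character with Enhanced Input movement, look, jump, sprint, slide and a first/third-person camera toggle.
; Move applies yaw-relative input and flags backward running, which blocks sprinting; sprint swaps the walk speed.
; Slide requires sprinting on the ground, launches along current velocity and starts a short timer.
; Jumping is blocked while sliding or jumping, with the jump flag clearing shortly after landing.
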(event Custom|StopSliding
  (Variables|Default|SetIsSliding false))

(event Input|EnhancedActionEvents|EnhancedInputActionIA_Move
  (params (ActionValue :type Vector%202D%20Structure) (ElapsedSeconds :type Float%20%28double-precision%29) (TriggeredSeconds :type Float%20%28double-precision%29) (InputAction :type Input%20Action%20Object%20Reference :default "/Game/TestGame/Input/Actions/IA_Move.IA_Move"))
  (CallFunction|Move (.x ActionValue) (.y ActionValue)))

(event Input|EnhancedActionEvents|EnhancedInputActionIA_Look
  (params (ActionValue :type Vector%202D%20Structure) (ElapsedSeconds :type Float%20%28double-precision%29) (TriggeredSeconds :type Float%20%28double-precision%29) (InputAction :type Input%20Action%20Object%20Reference :default "/Game/TestGame/Input/Actions/IA_Look.IA_Look"))
  (CallFunction|Look (.x ActionValue) (.y ActionValue)))

(event Input|EnhancedActionEvents|EnhancedInputActionIA_SwitchView
  (params (ActionValue :type Boolean) (ElapsedSeconds :type Float%20%28double-precision%29) (TriggeredSeconds :type Float%20%28double-precision%29) (InputAction :type Input%20Action%20Object%20Reference :default "/Game/TestGame/Input/Actions/IA_SwitchView.IA_SwitchView"))
  (:Started
    (Utilities|FlowControl|FlipFlop
      (:A
        (Components|Activation|SetActive (Variables|Default|GetFirstPersonCamera) true false)
        (Components|Activation|SetActive (Variables|Default|GetThirdPersonCamera) false false))
      (:B
        (Components|Activation|SetActive (Variables|Default|GetFirstPersonCamera) false false)
        (Components|Activation|SetActive (Variables|Default|GetThirdPersonCamera) true false)))))

(event Input|EnhancedActionEvents|EnhancedInputActionIA_Jump
  (params (ActionValue :type Boolean) (ElapsedSeconds :type Float%20%28double-precision%29) (TriggeredSeconds :type Float%20%28double-precision%29) (InputAction :type Input%20Action%20Object%20Reference :default "/Game/TestGame/Input/Actions/IA_Jump.IA_Jump"))
  (:Started
    (if (and (not (Variables|Default|GetIsJumping)) (not (Variables|Default|GetIsSliding)))
      (Character|Jump)))
  (:Canceled
    (Character|StopJumping :!label _label))
  (:Completed
    (goto _label)))

(event Input|EnhancedActionEvents|EnhancedInputActionIA_Sprint
  (params (ActionValue :type Boolean) (ElapsedSeconds :type Float%20%28double-precision%29) (TriggeredSeconds :type Float%20%28double-precision%29) (InputAction :type Input%20Action%20Object%20Reference :default "/Game/TestGame/Input/Actions/IA_Sprint.IA_Sprint"))
  (:Triggered
    (if (not (Variables|Default|GetIsRunningBackwards))
      (Variables|/Script/Engine.CharacterMovementComponent|SetMaxWalkSpeed (Variables|Character|GetCharacterMovement) (Variables|Default|GetSprintWalkingSpeed))
      (Variables|Default|SetIsSprinting true)
      (else
        (Variables|/Script/Engine.CharacterMovementComponent|SetMaxWalkSpeed (Variables|Character|GetCharacterMovement) (Variables|Default|GetDefaultWalkingSpeed) :!label _label)
        (Variables|Default|SetIsSprinting false))))
  (:Completed
    (goto _label)))

(event Input|EnhancedActionEvents|EnhancedInputActionIA_Slide
  (params (ActionValue :type Boolean) (ElapsedSeconds :type Float%20%28double-precision%29) (TriggeredSeconds :type Float%20%28double-precision%29) (InputAction :type Input%20Action%20Object%20Reference :default "/Game/TestGame/Input/Actions/IA_Slide.IA_Slide"))
  (:Started
    (if (and (Variables|Default|GetIsSprinting) (not (AI|Components|NavMovement|IsFalling (Variables|Character|GetCharacterMovement))))
      (Variables|Default|SetIsSliding true)
      (Character|LaunchCharacter (* (Math|Vector|Normalize (Transformation|GetVelocity)) 1e+03) false false)
      (Utilities|Time|SetTimerbyEvent (EventDispatchers|CreateEvent :!event Custom|StopSliding) 0.3))))

(event EventOnJumped
  (Variables|Default|SetIsJumping true))

(event EventOnLanded
  (params (Hit :type Hit%20Result%20Structure%20%28by%20ref%29))
  (Utilities|FlowControl|Delay 0.3)
  (Variables|Default|SetIsJumping false))

(fn ConstructionScript)

(fn Move
  (params (XAxis :type Float%20%28single-precision%29) (YAxis :type Float%20%28single-precision%29))
  (bind _returnvalue (Pawn|GetControlRotation :!class /Script/Engine.Pawn))
  (Pawn|Input|AddMovementInput (Math|Vector|GetRightVector (Math|Rotator|MakeRotator (.roll _returnvalue) 0.0 (.yaw _returnvalue))) XAxis false)
  (Pawn|Input|AddMovementInput (Math|Vector|GetForwardVector (Math|Rotator|MakeRotator 0.0 0.0 (.yaw (Pawn|GetControlRotation :!class /Script/Engine.Pawn)))) YAxis false)
  (Variables|Default|SetIsRunningBackwards (<= YAxis -1.0)))

(fn Look
  (params (XAxis :type Float%20%28single-precision%29) (YAxis :type Float%20%28single-precision%29))
  (Pawn|Input|AddControllerYawInput XAxis)
  (Pawn|Input|AddControllerPitchInput YAxis))