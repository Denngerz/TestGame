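; Energy rifle weapon that BP_MainUnit picks up on interaction and fires as a projectile weapon.
; Shoot checks CanShoot, then spends ammo, plays a sound and spawns the projectile; Reload refills to max capacity with its own sound.
; Projectiles spawn at ShootPoint, rotated toward a distant point along the owning unit's current camera forward vector, so shots follow the view without a trace.
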(event EventReload
  (Class|WeaponBase|SetCurrentBulletsAmount (Variables|Default|GetMaxAmmoCapacity))
  (Audio|PlaySound2D (Variables|Default|GetReloadSound) 1.0 1.0 0.0 0 0))

(event EventInteract
  (params (Interactor :type Actor%20Object%20Reference))
  (bind _asbp_main_unit (Utilities|Casting|CastToBP_MainUnit Interactor))
  (Default|PickUpWeapon _asbp_main_unit self))

(event EventShoot
  (bind _returnvalue (Class|WeaponBase|CanShoot))
  (if _returnvalue
    (Class|WeaponBase|DecreaseBulletsAmmount)
    (Audio|PlaySound2D (Variables|Default|GetShootSound) 1.0 1.0 0.0 0 0)
    (CallFunction|SpawnProjectile)))

(fn ConstructionScript)

(fn SpawnProjectile
  (bind _shootpoint (Variables|Default|GetShootPoint))
  (bind _returnvalue (Transformation|GetWorldLocation _shootpoint))
  (bind _asbp_main_unit (Utilities|Casting|CastToBP_MainUnit (Components|GetOwner)))
  (Game|SpawnActorfromClass (Variables|Default|GetProjectileClass) (Math|Transform|MakeTransform _returnvalue (Math|Rotator|FindLookatRotation _returnvalue (+ (Transformation|GetWorldLocation (Variables|/Game/TestGame/Blueprints/Characters/BP_MainUnit.BP_MainUnit_C|GetCurrentCamera _asbp_main_unit)) (* (Math|Vector|GetForwardVector (Variables|/Game/TestGame/Blueprints/Characters/BP_MainUnit.BP_MainUnit_C|GetCurrentCamera _asbp_main_unit)) 1e+04))) "1.000000,1.000000,1.000000") "AdjustIfPossibleButAlwaysSpawn" "MultiplyWithRoot" self 0))