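; Player character with parkour movement (sprint, slide, wall run, climbing), switchable first/third-person cameras, interaction and weapon handling.
; Wall runs start from hit events and use a plane constraint with lowered gravity; climbing switches to flying mode, guided by three forward line traces.
; WeaponsHolder stores weapon classes per slot; the selected one is spawned on a hand socket, and swapping or hiding destroys that actor.
; Health depletion only prints a message.
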(event Custom|Climb
  (params (WorldDirection :type Vector) (ScaleValue :type Float%20%28single-precision%29))
  ;[0.15 0.15 0.15 0.5 40] Climbing
  (bind (_foundwalltoclimb _hit) (Climbing|CheckforClimbingSurface))
  (if _foundwalltoclimb
    (Pawn|Input|AddMovementInput WorldDirection ScaleValue false)
    (Transformation|SetActorRotation (Math|Rotator|MakeRotfromX (* (.Normal (Collision|BreakHitResult _hit)) -1.0)))
    (else
      (CallFunction|StopClimbing))))

(event Custom|StopClimbing
  ;[0.15 0.15 0.15 0.5 40] Climbing
  (Pawn|Components|CharacterMovement|SetMovementMode (Variables|Character|GetCharacterMovement) "MOVE_Walking" 0)
  (Variables|State|SetIsClimbing false)
  (Variables|/Script/Engine.CharacterMovementComponent|SetbUseControllerDesiredRotation (Variables|Character|GetCharacterMovement) true)
  (if (Variables|Default|GetShouldToggleFPV)
    (View|ToggleFirstPersonView)))

(event Custom|StopSliding
  ;[0.15 0.15 0.15 0.5 40] Slide
  (Character|UnCrouch)
  (Variables|State|SetIsSliding false)
  (Utilities|FlowControl|Delay (Variables|Cooldown|GetSlideCooldownTime))
  (Variables|State|SetCanSlide true))

(event Custom|OnOutOfHealth
  (Development|PrintString "I am dead"))

(event Input|EnhancedActionEvents|EnhancedInputActionIA_Move
  (params (ActionValue :type Vector%202D%20Structure) (ElapsedSeconds :type Float%20%28double-precision%29) (TriggeredSeconds :type Float%20%28double-precision%29) (InputAction :type Input%20Action%20Object%20Reference :default "/Game/TestGame/Input/Actions/IA_Move.IA_Move"))
  ;[0.15 0.15 0.15 0.5 40] Movement
  ;;[0.4735 0.4735 0.4735 0.502 40] Move/Look
  (if (not (Variables|State|GetIsClimbing))
    (Movement|Move (.x ActionValue) (.y ActionValue))
    (WallRun|ValidateWallRun)
    (else
      (CallFunction|Climb (Transformation|GetActorRightVector) (.x ActionValue))
      (CallFunction|Climb (Transformation|GetActorUpVector) (.y ActionValue)))))

(event Input|EnhancedActionEvents|EnhancedInputActionIA_Look
  (params (ActionValue :type Vector%202D%20Structure) (ElapsedSeconds :type Float%20%28double-precision%29) (TriggeredSeconds :type Float%20%28double-precision%29) (InputAction :type Input%20Action%20Object%20Reference :default "/Game/TestGame/Input/Actions/IA_Look.IA_Look"))
  ;[0.15 0.15 0.15 0.5 40] Movement
  ;;[0.4735 0.4735 0.4735 0.502 40] Move/Look
  (Movement|Look (.x ActionValue) (.y ActionValue)))

(event Input|EnhancedActionEvents|EnhancedInputActionIA_OpenSecondSlot
  (params (ActionValue :type Boolean) (ElapsedSeconds :type Float%20%28double-precision%29) (TriggeredSeconds :type Float%20%28double-precision%29) (InputAction :type Input%20Action%20Object%20Reference :default "/Game/TestGame/Input/Actions/IA_OpenSecondSlot.IA_OpenSecondSlot"))
  (:Started
    (Weapon|SelectWeaponfromIndex 1)))

(event Input|EnhancedActionEvents|EnhancedInputActionIA_ToggleWeapon
  (params (ActionValue :type Boolean) (ElapsedSeconds :type Float%20%28double-precision%29) (TriggeredSeconds :type Float%20%28double-precision%29) (InputAction :type Input%20Action%20Object%20Reference :default "/Game/TestGame/Input/Actions/IA_ToggleWeapon.IA_ToggleWeapon"))
  (:Started
    (Utilities|FlowControl|FlipFlop
      (:A
        (Variables|State|SetIsHidingWeapon true)
        (Weapon|DetachWeapon))
      (:B
        (Variables|State|SetIsHidingWeapon false)
        (Weapon|AttachWeapon (.weapon (Variables|Weapon|GetCurrentChosenSlot)))))))

(event Input|EnhancedActionEvents|EnhancedInputActionIA_Reload
  (params (ActionValue :type Boolean) (ElapsedSeconds :type Float%20%28double-precision%29) (TriggeredSeconds :type Float%20%28double-precision%29) (InputAction :type Input%20Action%20Object%20Reference :default "/Game/TestGame/Input/Actions/IA_Reload.IA_Reload"))
  (bind _currentweapon (Variables|Weapon|GetCurrentWeapon))
  (:Started
    (Utilities|IsValid _currentweapon
      (:Is%20Valid
        (Class|WeaponBase|Reload _currentweapon)))))

(event Input|EnhancedActionEvents|EnhancedInputActionIA_SwitchView
  (params (ActionValue :type Boolean) (ElapsedSeconds :type Float%20%28double-precision%29) (TriggeredSeconds :type Float%20%28double-precision%29) (InputAction :type Input%20Action%20Object%20Reference :default "/Game/TestGame/Input/Actions/IA_SwitchView.IA_SwitchView"))
  (:Started
    (if (not (Variables|State|GetIsClimbing))
      (Utilities|FlowControl|FlipFlop
        (:A
          (View|ToggleFirstPersonView))
        (:B
          (View|ToggleThirdPersonView))))))

(event Input|EnhancedActionEvents|EnhancedInputActionIA_Jump
  (params (ActionValue :type Boolean) (ElapsedSeconds :type Float%20%28double-precision%29) (TriggeredSeconds :type Float%20%28double-precision%29) (InputAction :type Input%20Action%20Object%20Reference :default "/Game/TestGame/Input/Actions/IA_Jump.IA_Jump"))
  ;[0.15 0.15 0.15 0.5 40] Movement
  ;;[0.4735 0.4735 0.4735 0.502 40] Jumping
  (:Started
    (if (Variables|State|GetIsWallRunning)
      (WallRun|JumpfromWall)
      (elif (and (not (Variables|State|GetIsSliding)) (Variables|State|GetIsAbleToJump))
        (Development|PrintString "Hello")
        (Character|Jump)
        (Variables|State|SetIsAbleToJump false))))
  (:Canceled
    (Character|StopJumping :!label _label))
  (:Completed
    (goto _label)))

(event Input|EnhancedActionEvents|EnhancedInputActionIA_Sprint
  (params (ActionValue :type Boolean) (ElapsedSeconds :type Float%20%28double-precision%29) (TriggeredSeconds :type Float%20%28double-precision%29) (InputAction :type Input%20Action%20Object%20Reference :default "/Game/TestGame/Input/Actions/IA_Sprint.IA_Sprint"))
  (:Triggered
    (if (not (Variables|State|GetIsRunningBackwards))
      (Variables|/Script/Engine.CharacterMovementComponent|SetMaxWalkSpeed (Variables|Character|GetCharacterMovement) (Variables|Default|GetSprintWalkingSpeed))
      (Variables|State|SetIsSprinting true)
      (else
        (Variables|/Script/Engine.CharacterMovementComponent|SetMaxWalkSpeed (Variables|Character|GetCharacterMovement) (Variables|Default|GetDefaultWalkingSpeed) :!label _label)
        (Variables|State|SetIsSprinting false))))
  (:Completed
    (goto _label)))

(event Input|EnhancedActionEvents|EnhancedInputActionIA_Slide
  (params (ActionValue :type Boolean) (ElapsedSeconds :type Float%20%28double-precision%29) (TriggeredSeconds :type Float%20%28double-precision%29) (InputAction :type Input%20Action%20Object%20Reference :default "/Game/TestGame/Input/Actions/IA_Slide.IA_Slide"))
  ;[0.15 0.15 0.15 0.5 40] Slide
  (:Started
    (if (Math|Boolean|ANDBoolean (Variables|State|GetIsSprinting) (not (AI|Components|NavMovement|IsFalling (Variables|Character|GetCharacterMovement))) (Variables|State|GetCanSlide))
      (Variables|State|SetCanSlide false)
      (Variables|State|SetIsSliding true)
      (Character|LaunchCharacter (* (Math|Vector|Normalize (Transformation|GetVelocity)) 1e+03) false false)
      (Character|Crouch)
      (Utilities|Time|SetTimerbyEvent (EventDispatchers|CreateEvent :!event Custom|StopSliding) 0.3))))

(event Input|EnhancedActionEvents|EnhancedInputActionIA_Climb
  (params (ActionValue :type Boolean) (ElapsedSeconds :type Float%20%28double-precision%29) (TriggeredSeconds :type Float%20%28double-precision%29) (InputAction :type Input%20Action%20Object%20Reference :default "/Game/TestGame/Input/Actions/IA_Climb.IA_Climb"))
  ;[0.15 0.15 0.15 0.5 40] Climbing
  (:Started
    (if (not (Variables|State|GetIsClimbing))
      (bind (_foundwalltoclimb _hit) (Climbing|CheckforClimbingSurface))
      (if _foundwalltoclimb
        (Variables|/Script/Engine.CharacterMovementComponent|SetbUseControllerDesiredRotation (Variables|Character|GetCharacterMovement) false)
        (Variables|Default|SetShouldToggleFPV (Components|Activation|IsActive (Variables|Default|GetFirstPersonCamera)))
        (View|ToggleThirdPersonView)
        (Pawn|Components|CharacterMovement|SetMovementMode (Variables|Character|GetCharacterMovement) "MOVE_Flying" 0)
        (Components|MoveComponentTo (Variables|Default|GetCapsuleComponent) (+ (.Location (Collision|BreakHitResult _hit)) (* (.Normal (Collision|BreakHitResult _hit)) (Variables|/Script/Engine.CapsuleComponent|GetCapsuleRadius (Variables|Default|GetCapsuleComponent)))) (Math|Rotator|MakeRotfromX (* (.Normal (Collision|BreakHitResult _hit)) -1.0)) false false 0.2 false)
        (Variables|State|SetIsClimbing true))
      (else
        (CallFunction|StopClimbing)))))

(event Input|EnhancedActionEvents|EnhancedInputActionIA_Interact
  (params (ActionValue :type Boolean) (ElapsedSeconds :type Float%20%28double-precision%29) (TriggeredSeconds :type Float%20%28double-precision%29) (InputAction :type Input%20Action%20Object%20Reference :default "/Game/TestGame/Input/Actions/IA_Interact.IA_Interact"))
  (:Started
    (CallFunction|TryInteract)))

(event Input|EnhancedActionEvents|EnhancedInputActionIA_OpenFirstSlot
  (params (ActionValue :type Boolean) (ElapsedSeconds :type Float%20%28double-precision%29) (TriggeredSeconds :type Float%20%28double-precision%29) (InputAction :type Input%20Action%20Object%20Reference :default "/Game/TestGame/Input/Actions/IA_OpenFirstSlot.IA_OpenFirstSlot"))
  (:Started
    (Weapon|SelectWeaponfromIndex)))

(event Input|EnhancedActionEvents|EnhancedInputActionIA_Shoot
  (params (ActionValue :type Boolean) (ElapsedSeconds :type Float%20%28double-precision%29) (TriggeredSeconds :type Float%20%28double-precision%29) (InputAction :type Input%20Action%20Object%20Reference :default "/Game/TestGame/Input/Actions/IA_Shoot.IA_Shoot"))
  (bind _currentweapon (Variables|Weapon|GetCurrentWeapon))
  (:Started
    (Utilities|IsValid _currentweapon
      (:Is%20Valid
        (Class|WeaponBase|Shoot _currentweapon)))))

(event Collision|EventHit
  (params (MyComp :type Primitive%20Component%20Object%20Reference) (Other :type Actor%20Object%20Reference) (OtherComp :type Primitive%20Component%20Object%20Reference) (bSelfMoved :type Boolean) (HitLocation :type Vector :default "0, 0, 0") (HitNormal :type Vector :default "0, 0, 0") (NormalImpulse :type Vector :default "0, 0, 0") (Hit :type Hit%20Result%20Structure%20%28by%20ref%29))
  ;[0.15 0.15 0.15 0.5 40] Climbing
  (if (.CanWallRun (Climbing|CheckforWall Hit))
    (WallRun|StartWallRun HitNormal)
    (else
      (WallRun|StopWallRun))))

(event EventBeginPlay
  (View|ToggleThirdPersonView)
  (EventDispatchers|BindEventtoOnOutOfHealth (Variables|Default|GetHealthComponent) (EventDispatchers|CreateEvent :!event Custom|OnOutOfHealth)))

(event EventOnLanded
  (params (Hit :type Hit%20Result%20Structure%20%28by%20ref%29))
  ;[0.15 0.15 0.15 0.5 40] Movement
  ;;[0.4735 0.4735 0.4735 0.502 40] Jumping
  (WallRun|StopWallRun)
  (Variables|State|SetIsWallRunning false)
  (Utilities|FlowControl|Delay (Variables|Cooldown|GetJumpCooldownTime))
  (Variables|State|SetIsAbleToJump true))

(fn ConstructionScript)

(fn Move
  (params (XAxis :type Float%20%28single-precision%29) (YAxis :type Float%20%28single-precision%29))
  (bind _returnvalue (Pawn|GetControlRotation :!class /Script/Engine.Pawn))
  (Pawn|Input|AddMovementInput (Math|Vector|GetRightVector (Math|Rotator|MakeRotator (.roll _returnvalue) 0.0 (.yaw _returnvalue))) XAxis false)
  (Pawn|Input|AddMovementInput (Math|Vector|GetForwardVector (Math|Rotator|MakeRotator 0.0 0.0 (.yaw (Pawn|GetControlRotation :!class /Script/Engine.Pawn)))) YAxis false)
  (Variables|State|SetIsRunningBackwards (<= YAxis -1.0)))

(fn Look
  (params (XAxis :type Float%20%28single-precision%29) (YAxis :type Float%20%28single-precision%29))
  (Pawn|Input|AddControllerYawInput XAxis)
  (Pawn|Input|AddControllerPitchInput YAxis))

(fn StartWallRun
  (params (PlaneNormal :type Vector))
  (bind _charactermovement (Variables|Character|GetCharacterMovement))
  (if (and (AI|Components|NavMovement|IsFalling (Variables|Character|GetCharacterMovement)) (not (Variables|State|GetIsWallRunning)))
    (Class|MovementComponent|SetPlaneConstraintEnabled _charactermovement true)
    (Class|MovementComponent|SetPlaneConstraintNormal _charactermovement PlaneNormal)
    (Variables|/Script/Engine.CharacterMovementComponent|SetGravityScale (Variables|Character|GetCharacterMovement) 0.2)
    (bind _returnvalue (Utilities|Time|SetTimerbyEvent (EventDispatchers|CreateEvent :!event StopWallRun) 0.5))
    (Variables|Default|SetWallRunTimer _returnvalue)
    (Variables|State|SetIsWallRunning true)
    (Character|LaunchCharacter (* (Math|Vector|Normalize (Transformation|GetVelocity)) 8e+02) false false)))

(fn StopWallRun
  (bind _wallruntimer (Variables|Default|GetWallRunTimer))
  (Class|MovementComponent|SetPlaneConstraintEnabled (Variables|Character|GetCharacterMovement) false)
  (Variables|/Script/Engine.CharacterMovementComponent|SetGravityScale (Variables|Character|GetCharacterMovement) 1.0)
  (Utilities|Time|PauseTimerbyHandle _wallruntimer)
  (Utilities|Time|ClearandInvalidateTimerbyHandle _wallruntimer))

(fn CheckforWall
  (params (Hit :type Hit%20Result%20Structure%20%28by%20ref%29))
  (return Hit (and (> (Math|Float|Absolute(Float) (Math|Vector|DotProduct (.Normal (Collision|BreakHitResult Hit)) (Transformation|GetActorRightVector))) 0.8) (AI|Components|NavMovement|IsFalling (Variables|Character|GetCharacterMovement)))))

(fn ValidateWallRun
  (if (and (< (Math|Vector|VectorLength (Transformation|GetVelocity)) 2e+03) (Variables|State|GetIsWallRunning))
    (WallRun|StopWallRun)))

(fn JumpfromWall
  (WallRun|StopWallRun)
  (Character|LaunchCharacter (Math|Vector|ClampVectorSize (+ (* (Class|MovementComponent|GetPlaneConstraintNormal (Variables|Character|GetCharacterMovement)) (* (Math|Vector|VectorLength (Transformation|GetVelocity)) 2.0)) "0.000000,0.000000,150.000000") 0.0 1e+03) false false)
  (Variables|State|SetIsWallRunning false))

(fn CheckforClimbingSurface
  (bind _leftclimbtracestart (Variables|Default|GetLeftClimbTraceStart))
  (bind _centerclimbtracestart (Variables|Default|GetCenterClimbTraceStart))
  (bind _rightclimbtracestart (Variables|Default|GetRightClimbTraceStart))
  (bind _returnvalue (Transformation|GetWorldLocation _centerclimbtracestart))
  (bind _returnvalue_2 (Transformation|GetWorldLocation _leftclimbtracestart))
  (bind _returnvalue_3 (Transformation|GetWorldLocation _rightclimbtracestart))
  (LocalVariables|SetForwardVector (* (Transformation|GetActorForwardVector) 1e+02))
  (bind _outhit (Collision|LineTraceForObjects _returnvalue_2 (+ _returnvalue_2 (LocalVariables|GetForwardVector)) (Utilities|Array|MakeArray "ObjectTypeQuery1") false 0 "None"))
  (LocalVariables|SetLeftHitActor (.HitActor (Collision|BreakHitResult _outhit)))
  (bind _outhit_2 (Collision|LineTraceForObjects _returnvalue_3 (+ _returnvalue_3 (LocalVariables|GetForwardVector)) (Utilities|Array|MakeArray "ObjectTypeQuery1") false 0 "None"))
  (LocalVariables|SetRightHitActor (.HitActor (Collision|BreakHitResult _outhit_2)))
  (bind _outhit_3 (Collision|LineTraceForObjects _returnvalue (+ _returnvalue (LocalVariables|GetForwardVector)) (Utilities|Array|MakeArray "ObjectTypeQuery1") false 0 "None"))
  (bind _output_get (LocalVariables|SetCenterHitActor (.HitActor (Collision|BreakHitResult _outhit_3))))
  (return (and (Utilities|IsValid _output_get) (or (== (LocalVariables|GetRightHitActor) _output_get) (== (LocalVariables|GetLeftHitActor) _output_get))) _outhit_3))

(fn ToggleFirstPersonView
  (bind _firstpersoncamera (Variables|Default|GetFirstPersonCamera))
  (Components|Activation|SetActive _firstpersoncamera true false)
  (Components|Activation|SetActive (Variables|Default|GetThirdPersonCamera) false false)
  (Variables|Default|SetCurrentCamera _firstpersoncamera))

(fn ToggleThirdPersonView
  (bind _thirdpersoncamera (Variables|Default|GetThirdPersonCamera))
  (Components|Activation|SetActive (Variables|Default|GetFirstPersonCamera) false false)
  (Components|Activation|SetActive _thirdpersoncamera true false)
  (Variables|Default|SetCurrentCamera _thirdpersoncamera))

(fn TryInteract
  (bind _currentcamera (Variables|Default|GetCurrentCamera))
  (if (not (Variables|State|GetIsClimbing))
    (bind (_outhit _returnvalue) (Collision|SphereTraceForObjects (Transformation|GetActorLocation) (+ (Transformation|GetWorldLocation _currentcamera) (* (Math|Vector|GetForwardVector _currentcamera) 3.5e+02)) 3e+01 (Utilities|Array|MakeArray "ObjectTypeQuery7") false 0 "None"))
    (if _returnvalue
      (Class|InteractionInterface|Interact(Message) (.HitActor (Collision|BreakHitResult _outhit)) self))))

(fn PickUpWeapon
  (params (NewWeapon :type Weapon%20Base%20Object%20Reference))
  (bind _returnvalue (Class|WeaponsHolder|EmptySlotsLeft (Variables|Default|GetWeaponsHolder)))
  (if _returnvalue
    (bind _returnvalue_2 (Class|WeaponsHolder|TryAddWeapon (Variables|Default|GetWeaponsHolder) NewWeapon))
    (if (!= _returnvalue_2 -1)
      (Actor|DestroyActor NewWeapon)
      (if (== _returnvalue_2 (.index (Variables|Weapon|GetCurrentChosenSlot)))
        (Weapon|UpdateChosenWeaponSlot)
        (if (not (Variables|State|GetIsHidingWeapon))
          (Weapon|AttachWeapon (.weapon (Variables|Weapon|GetCurrentChosenSlot))))))
    (else
      (Weapon|DetachWeapon)
      (Weapon|DropWeapon (Variables|Weapon|GetCurrentChosenSlot))
      (Class|WeaponsHolder|SetWeaponatIndex (Variables|Default|GetWeaponsHolder) NewWeapon (.index (Variables|Weapon|GetCurrentChosenSlot)))
      (Weapon|UpdateChosenWeaponSlot)
      (Actor|DestroyActor NewWeapon)
      (if (not (Variables|State|GetIsHidingWeapon))
        (Weapon|AttachWeapon (.weapon (Variables|Weapon|GetCurrentChosenSlot)))))))

(fn DropWeapon
  (params (WeaponClass :type Storage%20Weapon%20Structure))
  (bind (_weapon _currentammo _index) (Utilities|Struct|BreakStorageWeapon WeaponClass))
  (Game|SpawnActorfromClass _weapon (Math|Transform|MakeTransform (Transformation|GetActorLocation) "0, 0, 0" "1.000000,1.000000,1.000000") "AdjustIfPossibleButAlwaysSpawn" "MultiplyWithRoot" 0 0)
  (Class|WeaponsHolder|DropWeaponatIndex (Variables|Default|GetWeaponsHolder) _index))

(fn AttachWeapon
  (params (WeaponClass :type Weapon%20Base%20Class%20Reference))
  (bind _returnvalue (Game|SpawnActorfromClass WeaponClass (Math|Transform|MakeTransform (Transformation|GetActorLocation) "0, 0, 0" "1.000000,1.000000,1.000000") "Undefined" "MultiplyWithRoot" self 0))
  (Physics|SetSimulatePhysics (Variables|/Script/TestGame.WeaponBase|GetWeaponMesh _returnvalue) false)
  (Collision|SetCollisionEnabled (Variables|/Script/TestGame.WeaponBase|GetWeaponMesh _returnvalue) "NoCollision")
  (bind _output_get (Variables|Weapon|SetCurrentWeapon _returnvalue))
  (Transformation|AttachComponentToComponent _output_get (Variables|Character|GetMesh) "WeaponSocket" "SnapToTarget" "SnapToTarget" "SnapToTarget" true))

(fn UpdateChosenWeaponSlot
  (bind _returnvalue (Class|WeaponsHolder|GetWeaponatIndex (Variables|Default|GetWeaponsHolder) (.index (Variables|Weapon|GetCurrentChosenSlot))))
  (Variables|Weapon|SetCurrentChosenSlot _returnvalue))

(fn DetachWeapon
  (bind _currentweapon (Variables|Weapon|GetCurrentWeapon))
  (Utilities|IsValid (Variables|Weapon|GetCurrentWeapon)
    (:Is%20Valid
      (Variables|/Script/TestGame.WeaponBase|SetWeaponType _currentweapon "Unarmed")
      (Actor|DestroyActor _currentweapon))))

(fn UpdateWeaponinHands
  (Weapon|DetachWeapon)
  (Weapon|AttachWeapon (.weapon (Variables|Weapon|GetCurrentChosenSlot))))

(fn SelectWeaponfromIndex
  (params (Index :type Integer))
  (bind _returnvalue (Class|WeaponsHolder|GetWeaponatIndex (Variables|Default|GetWeaponsHolder) Index))
  (Variables|Weapon|SetCurrentChosenSlot _returnvalue)
  (if (not (Variables|State|GetIsHidingWeapon))
    (Weapon|UpdateWeaponinHands)))