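; AI controller for the attacking alien that runs its behavior tree on BeginPlay and tracks the player by sight.
; Perception updates go to HandleSightSense, which ignores non-sight stimuli and any actor other than the player character.
; Sensing the player sets the TargetActor blackboard key; losing sight clears it and stores the stimulus position in LastKnownLocation.
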(event OnTargetPerceptionUpdated(AIPerception)
  (params (Actor :type Actor%20Object%20Reference) (Stimulus :type AI%20Stimulus%20Structure))
  (CallFunction|HandleSightSense Actor Stimulus))

(event EventBeginPlay
  (AI|RunBehaviorTree (Variables|Default|GetBehaviorTreeToRun)))

(fn ConstructionScript)

(fn HandleSightSense
  (params (Actor :type Actor%20Object%20Reference) (Stimulus :type AI%20Stimulus%20Structure))
  (bind (_age _expirationage _strength _stimuluslocation _receiverlocation _tag _bsuccessfullysensed) (Utilities|Struct|BreakAIStimulus Stimulus))
  (bind _returnvalue (Class|AIPerceptionSystem|GetSenseClassforStimulus Stimulus))
  (if (== _returnvalue "/Script/AIModule.AISense_Sight")
    (if (== Actor (Game|GetPlayerCharacter 0))
      (AI|Components|Blackboard|SetValueasObject (Variables|Default|GetBlackboard) (Utilities|Name|MakeLiteralName "TargetActor") (Utilities|SelectObject (Game|GetPlayerCharacter 0) 0 _bsuccessfullysensed))
      (if (not _bsuccessfullysensed)
        (AI|Components|Blackboard|SetValueasVector (Variables|Default|GetBlackboard) (Utilities|Name|MakeLiteralName "LastKnownLocation") _stimuluslocation)))))