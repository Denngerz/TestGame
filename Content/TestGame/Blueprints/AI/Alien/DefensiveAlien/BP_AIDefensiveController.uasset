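; AI controller for the defensive alien enemy that runs a behavior tree and reacts to spotting the player.
; On BeginPlay it starts the configured behavior tree, and AI perception updates feed HandleSightSense.
; Successful sight of the player character writes it to the TargetActor blackboard key and prints a debug string.
; Losing sight does not clear the key.
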(event OnTargetPerceptionUpdated(AIPerception)
  (params (Actor :type Actor%20Object%20Reference) (Stimulus :type AI%20Stimulus%20Structure))
  (CallFunction|HandleSightSense Actor Stimulus))

(event EventBeginPlay
  (AI|RunBehaviorTree (Variables|Default|GetBehaviorTreeToRun)))

(fn ConstructionScript)

(fn HandleSightSense
  (params (Actor :type Actor%20Object%20Reference) (Stimulus :type AI%20Stimulus%20Structure))
  (bind _returnvalue (Class|AIPerceptionSystem|GetSenseClassforStimulus Stimulus))
  (if (== _returnvalue "/Script/AIModule.AISense_Sight")
    (if (== Actor (Game|GetPlayerCharacter 0))
      (if (.bSuccessfullySensed (Utilities|Struct|BreakAIStimulus Stimulus))
        (AI|Components|Blackboard|SetValueasObject (Variables|Default|GetBlackboard) (Utilities|Name|MakeLiteralName "TargetActor") (Game|GetPlayerCharacter 0))
        (Development|PrintString "Hello")))))