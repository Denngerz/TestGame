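; BP_SpawnActorTeminal is an interactable terminal that spawns a destructible box, allowing one live box at a time.
; On Interact, it spawns BP_DestructibleBox at the SpawnPoint of its referenced SpawnPlace and stores it in SpawnedActor.
; While that stored box is still valid, further interactions only play a Denied sound at the terminal's location.
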(event EventInteract
  (params (Interactor :type Actor%20Object%20Reference))
  (if (not (Utilities|IsValid (Variables|Default|GetSpawnedActor)))
    (bind _returnvalue (Game|SpawnActorfromClass "/Game/TestGame/Blueprints/Destructible/DestructibleBox/BP_DestructibleBox.BP_DestructibleBox_C" (Math|Transform|MakeTransform (Transformation|GetWorldLocation (Variables|/Game/TestGame/Blueprints/Interactable/SpawnActorTerminal/BP_SpawnPlace.BP_SpawnPlace_C|GetSpawnPoint (Variables|Default|GetSpawnPlace))) "0, 0, 0" "1.000000,1.000000,1.000000") "Undefined" "MultiplyWithRoot" 0 0))
    (Variables|Default|SetSpawnedActor _returnvalue)
    (else
      (Audio|PlaySoundatLocation "/Game/TestGame/Sounds/Denied.Denied" (Transformation|GetActorLocation) "0, 0, 0" 1.0 1.0 0.0 0 0 0 0))))

(fn ConstructionScript)