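; Spawner actor that periodically adds AI-controlled aliens to the level at random spawn points.
; On BeginPlay it caches the game state, gathers all BP_AISpawnPoint actors and starts a looping timer.
; TrySpawnAI asks BP_Gamemode whether spawning is allowed, then spawns a BP_Alien and a randomly chosen AI controller class at a random point's location, and has that controller possess the alien.
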(event Custom|TrySpawnAI
  (bind _asbp_gamemode (Utilities|Casting|CastToBP_Gamemode (Game|GetGameMode)))
  (bind _returnvalue (Class|TestGameGamemode|CanSpawnAI _asbp_gamemode))
  (if _returnvalue
    (bind _returnvalue_2 (CallFunction|GetRandomSpawnLocation))
    (bind _outitem (CallFunction|GetRandomAIControllerClass))
    (bind _returnvalue_3 (Game|SpawnActorfromClass "/Game/TestGame/Blueprints/AI/Alien/BP_Alien.BP_Alien_C" (Math|Transform|MakeTransform _returnvalue_2 "0, 0, 0" "1.000000,1.000000,1.000000") "Undefined" "MultiplyWithRoot" 0 0))
    (bind _returnvalue_4 (Game|SpawnActorfromClass _outitem (Math|Transform|MakeTransform _returnvalue_2 "0, 0, 0" "1.000000,1.000000,1.000000") "Undefined" "MultiplyWithRoot" 0 0))
    (Pawn|Possess _returnvalue_4 _returnvalue_3)))

(event EventBeginPlay
  (bind _astest_game_game_state (Utilities|Casting|CastToTestGameGameState (Game|GetGameState)))
  (Variables|Default|SetGamestate _astest_game_game_state)
  (bind _outactors (Actor|GetAllActorsOfClass "/Game/TestGame/Blueprints/AI/AISpawner/BP_AISpawnPoint.BP_AISpawnPoint_C"))
  (Variables|Default|SetSpawnPoints _outactors)
  (Utilities|Time|SetTimerbyEvent (EventDispatchers|CreateEvent :!event Custom|TrySpawnAI) 5.0 true false 1.0))

(fn ConstructionScript)

(fn GetRandomSpawnLocation
  (return (Transformation|GetWorldLocation (Variables|/Game/TestGame/Blueprints/AI/AISpawner/BP_AISpawnPoint.BP_AISpawnPoint_C|GetSpawnPoint (.OutItem (Utilities|Array|Random (Variables|Default|GetSpawnPoints)))))))

(fn GetRandomAIControllerClass
  (return (.OutItem (Utilities|Array|Random (Variables|Default|GetAIControllerClasses)))))