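; BP_HealBox is an interactable heal box that heals a BP_MainUnit interactor through the Gameplay Ability System.
; On Interact it applies the GE_Heal effect to the unit's ability system component and plays a heal sound at the box.
; A CanHeal flag and a one-second timer form a cooldown, and attempts during it play a denied sound instead.
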(event Custom|ResetHealing
  (Variables|Default|SetCanHeal true))

(event EventInteract
  (params (Interactor :type Actor%20Object%20Reference))
  (if (Variables|Default|GetCanHeal)
    (bind _asbp_main_unit (Utilities|Casting|CastToBP_MainUnit Interactor))
    (Utilities|IsValid (Ability|GetAbilitySystemComponent _asbp_main_unit)
      (:Is%20Valid
        (GameplayEffects|ApplyGameplayEffectToSelf :self (Ability|GetAbilitySystemComponent _asbp_main_unit) :GameplayEffectClass "/Game/TestGame/Blueprints/AbilitySystem/HealBox/GE_Heal.GE_Heal_C")
        (Audio|PlaySoundatLocation "/Game/TestGame/Sounds/HealSound.HealSound" (Transformation|GetActorLocation) "0, 0, 0" 1.0 1.0 0.0 0 0 0 0)
        (Variables|Default|SetCanHeal false)
        (Utilities|Time|SetTimerbyEvent (EventDispatchers|CreateEvent :!event Custom|ResetHealing) 1.0 false false 2.0)))
    (else
      (Audio|PlaySoundatLocation "/Game/TestGame/Sounds/Denied.Denied" (Transformation|GetActorLocation) "0, 0, 0" 1.0 1.0 0.0 0 0 0 0))))

(fn ConstructionScript)