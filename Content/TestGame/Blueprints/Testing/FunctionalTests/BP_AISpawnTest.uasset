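; BP_AISpawnTest is a functional test that checks whether BP_AISpawner can spawn AI.
; StartTest caches the level's spawner, the TestGameGameState and the BP_Gamemode, though the game mode is not used afterwards.
; A DoOnce on Tick calls TrySpawnAI, then immediately finishes the test as Succeeded if the game state's CurrentAICount is above zero, otherwise Failed.
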(event EventPrepareTest)

(event EventStartTest
  (bind _returnvalue (Actor|GetActorOfClass "/Game/TestGame/Blueprints/AI/AISpawner/BP_AISpawner.BP_AISpawner_C"))
  (Variables|Default|SetAISpawner _returnvalue)
  (bind _astest_game_game_state (Utilities|Casting|CastToTestGameGameState (Game|GetGameState)))
  (Variables|Default|SetGamestate _astest_game_game_state)
  (bind _asbp_gamemode (Utilities|Casting|CastToBP_Gamemode (Game|GetGameMode)))
  (Variables|Default|SetGamemode _asbp_gamemode))

(event EventTick
  (params (DeltaSeconds :type Float%20%28single-precision%29))
  (Utilities|FlowControl|DoOnce false
    (:Completed
      (Default|TrySpawnAI (Variables|Default|GetAISpawner))
      (if (> (Variables|/Script/TestGame.TestGameGameState|GetCurrentAICount (Variables|Default|GetGamestate)) 0)
        (Class|FunctionalTest|FinishTest "Succeeded")
        (else
          (Class|FunctionalTest|FinishTest "Failed"))))))

(fn ConstructionScript)