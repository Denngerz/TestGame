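; BP_AutomaticRifle is a pickup rifle weapon that BP_MainUnit collects through Interact.
; Shoot checks and spends ammo, plays muzzle effect and sound, then line traces from the owning unit's current camera.
; Hits on ability-system actors receive a GameplayEffect with set-by-caller damage and a blood effect, while other DamageableInterface actors get a damage message.
; Reload refills ammo to max capacity with a sound.
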(event EventReload
  (Class|WeaponBase|SetCurrentBulletsAmount (Variables|Default|GetMaxAmmoCapacity))
  (Audio|PlaySound2D (Variables|Default|GetReloadSound) 1.0 1.0 0.0 0 0))

(event EventInteract
  (params (Interactor :type Actor%20Object%20Reference))
  (bind _asbp_main_unit (Utilities|Casting|CastToBP_MainUnit Interactor))
  (Default|PickUpWeapon _asbp_main_unit self))

(event EventShoot
  (bind _returnvalue (Class|WeaponBase|CanShoot))
  (if _returnvalue
    (Class|WeaponBase|DecreaseBulletsAmmount)
    (Effects|SpawnEmitteratLocation "/Game/TestGame/VFX/Particles/Explosion/P_Explosion_Big_A.P_Explosion_Big_A" (Transformation|GetWorldLocation (Variables|Default|GetShootPoint)) "0, 0, 0" "0.010000,0.010000,0.010000")
    (Audio|PlaySound2D (Variables|Default|GetShootSound) 1.0 1.0 0.0 0 0)
    (bind (_outhit _returnvalue_2) (CallFunction|PerformShootTrace))
    (if _returnvalue_2
      (Utilities|IsValid (Ability|GetAbilitySystemComponent (.HitActor (Collision|BreakHitResult _outhit)))
        (:Is%20Valid
          (CallFunction|ApplyDamagetoASC (Ability|GetAbilitySystemComponent (.HitActor (Collision|BreakHitResult _outhit))))
          (Effects|SpawnEmitteratLocation "/Game/TestGame/VFX/Particles/Blood/P_Blood_Splat_Cone.P_Blood_Splat_Cone" (.Location (Collision|BreakHitResult _outhit)) "0, 0, 0" "0.500000,0.500000,0.500000"))
        (:Is%20Not%20Valid
          (if (Utilities|DoesObjectImplementInterface (.HitActor (Collision|BreakHitResult _outhit)) "/Script/TestGame.DamageableInterface")
            (Class|DamageableInterface|TakeDamage(Message) (.HitActor (Collision|BreakHitResult _outhit)) (Variables|Default|GetDamage) self)))))))

(fn ConstructionScript)

(fn ApplyDamagetoASC
  (params (TargetASC :type Ability%20System%20Component%20Object%20Reference))
  (bind _returnvalue (Ability|GameplayEffect|AssignTagSetbyCallerMagnitude (GameplayEffects|MakeOutgoingSpec :self TargetASC :GameplayEffectClass "/Game/TestGame/Blueprints/AbilitySystem/Weapons/GE_AutomaticRifleShot.GE_AutomaticRifleShot_C") "(TagName=\"Data.Damage\")" (* (Variables|Default|GetDamage) -1.0)))
  (GameplayEffects|ApplyGameplayEffectSpecToSelf TargetASC _returnvalue))

(fn PerformShootTrace
  (bind _asbp_main_unit (Utilities|Casting|CastToBP_MainUnit (Components|GetOwner)))
  (LocalVariables|SetCurrentCamera (Variables|/Game/TestGame/Blueprints/Characters/BP_MainUnit.BP_MainUnit_C|GetCurrentCamera _asbp_main_unit))
  (bind (_outhit _returnvalue) (Collision|LineTraceByChannel (Transformation|GetWorldLocation (Variables|/Game/TestGame/Blueprints/Characters/BP_MainUnit.BP_MainUnit_C|GetCurrentCamera _asbp_main_unit)) (+ (Transformation|GetWorldLocation (Variables|/Game/TestGame/Blueprints/Characters/BP_MainUnit.BP_MainUnit_C|GetCurrentCamera _asbp_main_unit)) (* (Math|Vector|GetForwardVector (Variables|/Game/TestGame/Blueprints/Characters/BP_MainUnit.BP_MainUnit_C|GetCurrentCamera _asbp_main_unit)) 1e+04)) "TraceTypeQuery2" false (Utilities|Array|MakeArray _asbp_main_unit) "None"))
  (return _outhit _returnvalue))